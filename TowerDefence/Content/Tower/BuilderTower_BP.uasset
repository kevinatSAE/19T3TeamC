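; BuilderTower_BP is a placement preview actor for building towers.
; Every tick it moves to the world-static surface hit under the player's cursor.
; Its PlaceTower event spawns a TowerBP at that transform, passes it TowerData and initializes it, deducts a fixed resource cost from ThirdPersonGameMode, then destroys itself.
; The deduction happens here without any affordability check.
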(event Custom|PlaceTower
  (bind _gamemode (Variables|Default|GetGamemode))
  ;[0.99 0.1568 1] Event Place and Spawn Tower
  (bind _returnvalue (Game|SpawnActorfromClass "/Game/Tower/Towerbp.TowerBP_C" (Transformation|GetActorTransform) "AlwaysSpawn" 0 0))
  (Variables|/Game/Tower/Towerbp.TowerBP_C|SetTowerStruc _returnvalue (Variables|Default|GetTowerData))
  (Default|TowerInt _returnvalue)
  (Variables|/Game/ThirdPersonBP/Blueprints/ThirdPersonGameMode.ThirdPersonGameMode_C|SetCurrentResources _gamemode (- (Variables|/Game/ThirdPersonBP/Blueprints/ThirdPersonGameMode.ThirdPersonGameMode_C|GetCurrentResources _gamemode) 10))
  (Actor|DestroyActor))

(event EventBeginPlay
  (bind _outactors (Actor|GetAllActorsOfClass "/Game/ThirdPersonBP/Blueprints/ThirdPersonGameMode.ThirdPersonGameMode_C"))
  (Variables|Default|SetGamemode (Utilities|Array|Get(acopy) _outactors)))

(event Collision|EventActorBeginOverlap
  (params (OtherActor :type Actor%20Object%20Reference)))

(event EventTick
  (params (DeltaSeconds :type Float%20%28single-precision%29))
  (bind _returnvalue (Game|GetPlayerController 0))
  (bind _array (Utilities|Array|MakeArray "ObjectTypeQuery1"))
  (bind (_hitresult _returnvalue_2) (Class|PlayerController|GetHitResultUnderCursorforObjects _returnvalue _array true))
  ;[1 1 1] Add Cursor and location after click build tower
  (if _returnvalue_2
    (Transformation|SetActorLocation (.Location (Collision|BreakHitResult _hitresult)) false false)))

(fn ConstructionScript)